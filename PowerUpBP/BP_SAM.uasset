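; BP_SAM is a powerup pickup that makes SAM the active powerup of the ThirdPersonCharacter that overlaps it.
; If the character's CoolDown flag is true, it clears the oil slick, invisibility and shield flags, sets SAM and destroys itself.
; It also refills the character's Ammo and passes the SAM flag and character to SetPower on top-level Pow_hud widgets to update the HUD.
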(event Collision|EventActorBeginOverlap
  (params (OtherActor :type Actor%20Object%20Reference))
  (bind _asthird_person_character (Utilities|Casting|CastToThirdPersonCharacter OtherActor))
  (if (Variables|/Game/PowerUpsBP/ThirdPersonBP/Blueprints/ThirdPersonCharacter.ThirdPersonCharacter_C|GetCoolDown _asthird_person_character)
    ;[1 1 1] set active powerup
    (Variables|/Game/PowerUpsBP/ThirdPersonBP/Blueprints/ThirdPersonCharacter.ThirdPersonCharacter_C|SetOilSlick _asthird_person_character false)
    (Variables|/Game/PowerUpsBP/ThirdPersonBP/Blueprints/ThirdPersonCharacter.ThirdPersonCharacter_C|SetHas%20Invisibility _asthird_person_character false)
    (Variables|/Game/PowerUpsBP/ThirdPersonBP/Blueprints/ThirdPersonCharacter.ThirdPersonCharacter_C|SetHAs%20Sheild _asthird_person_character false)
    (bind _output_get (Variables|/Game/PowerUpsBP/ThirdPersonBP/Blueprints/ThirdPersonCharacter.ThirdPersonCharacter_C|SetSAM _asthird_person_character true))
    (Actor|DestroyActor) ; Remove powerup
    (Variables|/Game/PowerUpsBP/ThirdPersonBP/Blueprints/ThirdPersonCharacter.ThirdPersonCharacter_C|SetAmmo _asthird_person_character 3.0)
    ;[1 0 0] set powerup to HUD
    (bind _foundwidgets (Widget|GetAllWidgetsOfClass "/Game/Pow_hud.Pow_hud_C" true))
    (Default|SetPower _foundwidgets _output_get _asthird_person_character)))

(fn ConstructionScript)