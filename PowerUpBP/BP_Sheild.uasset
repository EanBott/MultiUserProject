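; Shield power-up pickup that a ThirdPersonCharacter collects by overlapping it while that character's CoolDown flag is true.
; Pickup makes the shield the active power by setting its flag and clearing the SAM, invisibility and oil slick flags.
; It then destroys itself, sets the character's Ammo and calls SetPower on the top-level Pow_hud widgets to update the HUD.
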(event EventBeginPlay)

(event Collision|EventActorBeginOverlap
  (params (OtherActor :type Actor%20Object%20Reference))
  (bind _asthird_person_character (Utilities|Casting|CastToThirdPersonCharacter OtherActor))
  (if (Variables|/Game/PowerUpsBP/ThirdPersonBP/Blueprints/ThirdPersonCharacter.ThirdPersonCharacter_C|GetCoolDown _asthird_person_character)
    ;[1 1 1] set active powerUP
    (Variables|/Game/PowerUpsBP/ThirdPersonBP/Blueprints/ThirdPersonCharacter.ThirdPersonCharacter_C|SetSAM _asthird_person_character false)
    (Variables|/Game/PowerUpsBP/ThirdPersonBP/Blueprints/ThirdPersonCharacter.ThirdPersonCharacter_C|SetHas%20Invisibility _asthird_person_character false)
    (Variables|/Game/PowerUpsBP/ThirdPersonBP/Blueprints/ThirdPersonCharacter.ThirdPersonCharacter_C|SetOilSlick _asthird_person_character false)
    (bind _output_get (Variables|/Game/PowerUpsBP/ThirdPersonBP/Blueprints/ThirdPersonCharacter.ThirdPersonCharacter_C|SetHAs%20Sheild _asthird_person_character true))
    (Actor|DestroyActor) ; Remove powerUP
    (Variables|/Game/PowerUpsBP/ThirdPersonBP/Blueprints/ThirdPersonCharacter.ThirdPersonCharacter_C|SetAmmo _asthird_person_character 1.0)
    ;[1.482 0 0] set power to HUD
    (bind _foundwidgets (Widget|GetAllWidgetsOfClass "/Game/Pow_hud.Pow_hud_C" true))
    (Default|SetPower _foundwidgets _output_get _asthird_person_character)))

(event EventTick
  (params (DeltaSeconds :type Float%20%28single-precision%29)))

(fn ConstructionScript)